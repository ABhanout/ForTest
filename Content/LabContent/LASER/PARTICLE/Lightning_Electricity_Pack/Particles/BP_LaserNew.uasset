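; Laser beam actor that drives the Beam End parameter of its particle effect from forward line traces.
; On BeginPlay, a timeline extends the beam from the actor's location to the first Visibility hit.
; When it finishes, a gate opens so a trace every Tick keeps the endpoint updated.
; Only the world X coordinate of the hit is used, plus a fixed offset, with Y and Z left at zero.
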(event `self.ReceiveBeginPlay`
  (bind _defaultsceneroot (`self.DefaultSceneRoot`))
  (bind _returnvalue (`SceneComponent.K2_GetComponentLocation` _defaultsceneroot))
  (bind _outhit (`KismetSystemLibrary.LineTraceSingle` _returnvalue (+ _returnvalue (* (`SceneComponent.GetForwardVector` _defaultsceneroot) 50000.0)) "TraceTypeQuery1"))
  (bind (_direction _newtrack_0) (`Timeline|Timeline_0`)
    (:`Update`
      (bind _output_get (set `self.BeamEndV` (`KismetMathLibrary.MakeVector` (`KismetMathLibrary.Lerp` (.x _returnvalue) (.x (`.Location` (`GameplayStatics.BreakHitResult` _outhit))) _newtrack_0))))
      (`FXSystemComponent.SetVectorParameter` (`self.P_Lasernew`) "Beam End" (`KismetMathLibrary.MakeVector` (+ (.x _output_get) 725.0))))
    (:`Finished`
      (goto _label :!via `Open`))))

(event `self.ReceiveTick`
  (params (DeltaSeconds :type "Float (single-precision)"))
  (bind _defaultsceneroot (`self.DefaultSceneRoot`))
  (bind _returnvalue (`SceneComponent.K2_GetComponentLocation` _defaultsceneroot))
  (bind _outhit (`KismetSystemLibrary.LineTraceSingle` _returnvalue (+ _returnvalue (* (`SceneComponent.GetForwardVector` _defaultsceneroot) 50000.0)) "TraceTypeQuery1"))
  (`/Engine/EditorBlueprintResources/StandardMacros.Gate` true :!label _label
    (:`Exit`
      (bind _output_get (set `self.BeamEndV` (`KismetMathLibrary.MakeVector` (.x (`.Location` (`GameplayStatics.BreakHitResult` _outhit))))))
      (`FXSystemComponent.SetVectorParameter` (`self.P_Lasernew`) "Beam End" (`KismetMathLibrary.MakeVector` (+ (.x _output_get) 725.0))))))

(fn `UserConstructionScript`)